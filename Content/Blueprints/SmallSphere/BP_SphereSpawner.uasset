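; BP_SphereSpawner is an actor that keeps spawning BP_SmallSphere actors at random points within a radius around itself.
; On BeginPlay it starts a looping timer at the SpawnTime interval, and each tick of that timer spawns one sphere with a random rotation.
; The spawn point offsets the actor's location along a random direction by a random distance up to SpawnRadius, so spawns cluster toward the center.
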(event Custom|SpawnSmallSphere
  ;[0.1198 0 0] Start Sphere Spawn Timer
  (Game|SpawnActorfromClass "/Game/Blueprints/SmallSphere/BP_SmallSphere.BP_SmallSphere_C" (Math|Transform|MakeTransform (CallFunction|GetRandomPointinSphereRadius) (Math|Random|RandomRotator false) "1.000000,1.000000,1.000000") "Undefined" "MultiplyWithRoot" 0 0))

(event EventBeginPlay
  ;[0.1198 0 0] Start Sphere Spawn Timer
  (Utilities|Time|SetTimerbyEvent (delegate Custom|SpawnSmallSphere) (Variables|SphereSpawner|GetSpawnTime) true))

(fn ConstructionScript)

(fn GetRandomPointinSphereRadius
  (return (+ (Transformation|GetActorLocation) (* (Math|Vector|GetForwardVector (Math|Random|RandomRotator false)) (Math|Random|RandomFloatinRange 0.0 (Variables|SphereSpawner|GetSpawnRadius))))))