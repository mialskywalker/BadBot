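; BP_SmallSphere is a short-lived, drifting pickup that increments the BP_BadBotGameMode score when a Pawn overlaps it.
; Timelines scale the mesh as it winks in on spawn and out before destruction, triggered by overlap or a lifetime timer.
; Tick moves it along its forward vector while applying a random spin chosen at BeginPlay, so its path continually changes direction.
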(event Custom|WinkOut
  ;[0.1198 0 0] Start WinkOut Timeline
  (if (not (Variables|Default|GetIsWinking))
    (Variables|Default|SetIsWinking true)
    (bind _scale (Timeline|WinkOutTimeline Play)
      (:Update
        (CallFunction|ScaleSphere _scale))
      (:Finished
        (Actor|DestroyActor)))))

(event Custom|WinkIn
  ;[0.1198 0 0] Wink into Existence
  (bind _scale (Timeline|WinkInTimeline Play)
    (:Update
      (Transformation|SetWorldScale3D (Variables|Default|GetSphereMesh) _scale))))

(event Custom|OnSphereOverlap
  (params (OverlappedComponent :type Primitive%20Component%20Object%20Reference) (OtherActor :type Actor%20Object%20Reference) (OtherComp :type Primitive%20Component%20Object%20Reference) (OtherBodyIndex :type Integer) (bFromSweep :type Boolean) (SweepResult :type Hit%20Result%20Structure%20%28by%20ref%29))
  ;[0.1198 0 0] Handle Overlap
  (if (Class|GameplayStatics|ObjectIsA OtherActor "/Script/Engine.Pawn")
    (bind _asbp_bad_bot_game_mode (Utilities|Casting|CastToBP_BadBotGameMode (Game|GetGameMode)))
    (Default|IncrementScore _asbp_bad_bot_game_mode)
    (CallFunction|WinkOut)))

(event EventBeginPlay
  (CallFunction|Winkin)
  (CallFunction|InitializeDeltaRotation)
  ;[0.1198 0 0] Start WinkOut Timeline
  (Utilities|Time|SetTimerbyEvent (delegate Custom|WinkOut) (Variables|Default|GetLifetime))
  ;[0.1198 0 0] Handle Overlap
  (Collision|AssignOnComponentBeginOverlap (Variables|Default|GetSphereVolume) (delegate Custom|OnSphereOverlap)))

(event EventTick
  (params (DeltaSeconds :type Float%20%28single-precision%29))
  ;[0.2448 0.2448 0.2448] Update Location and Rotation
  (CallFunction|UpdateLocation DeltaSeconds)
  (CallFunction|UpdateRotation DeltaSeconds))

(fn ConstructionScript)

(fn InitializeDeltaRotation
  (Variables|Default|SetDelta%20Rotation (* (Math|Random|RandomRotator false) (Variables|SphereMovement|GetRotationScaleFactor))))

(fn UpdateLocation
  (params (DeltaTime :type Float%20%28double-precision%29))
  (Transformation|AddActorWorldOffset (* (Transformation|GetActorForwardVector) (* DeltaTime (Variables|SphereMovement|GetSpeed)))))

(fn UpdateRotation
  (params (DeltaSeconds :type Float%20%28single-precision%29))
  (Class|Actor|AddActorWorldRotation (* (Variables|Default|GetDelta%20Rotation) DeltaSeconds)))

(fn ScaleSphere
  (params (Scale :type Float%20%28single-precision%29))
  (Transformation|SetWorldScale3D (Variables|Default|GetSphereMesh) (Math|Vector|MakeVector Scale Scale Scale)))